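; BP_Interact is an interaction point actor that shows an icon when the player is near and relays interactions to its parent actor.
; On BeginPlay it creates a small WBP_InteractIcon in the viewport with a reference back to itself.
; Tick checks player distance and plays or reverses a Timeline that drives the icon's opacity.
; InteractChildObject forwards to a valid parent actor through InteractObjectMessage, suggesting use as a child actor.
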(event Custom|Widegt
  (bind _returnvalue (UserInterface|CreateWidget "/Game/Tello/Widgets/WBP_InteractIcon.WBP_InteractIcon_C"))
  (Variables|Default|SetNewVar _returnvalue)
  (Variables|/Game/Tello/Widgets/WBP_InteractIcon.WBP_InteractIcon_C|SetParentActor (Variables|Default|GetNewVar) self)
  (UserInterface|Viewport|AddtoViewport (Variables|Default|GetNewVar) -1)
  (Class|UserWidget|SetDesiredSizeinViewport (Variables|Default|GetNewVar) "(X=32.000000,Y=32.000000)"))

(event EventBeginPlay
  (CallFunction|Widegt))

(event Collision|EventActorBeginOverlap
  (params (OtherActor :type Actor%20Object%20Reference)))

(event EventInteractChildObject
  (bind _returnvalue (Actor|GetParentActor))
  (Utilities|IsValid _returnvalue
    (:Is%20Valid
      (Class|BPIInteractObjects|InteractObject(Message) _returnvalue))))

(event EventTick
  (params (DeltaSeconds :type Float%20%28single-precision%29))
  (if (<= (Transformation|GetDistanceTo (Game|GetPlayerCharacter 0)) 3e+02)
    (bind _newtrack_0 (Timeline|Timeline Play)
      (:Update
        (Variables|/Script/UMG.Widget|SetRenderOpacity (Variables|Default|GetNewVar) _newtrack_0)))
    (else
      (Timeline|Timeline Reverse))))

(fn ConstructionScript)