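; BP_Door is a door actor that swings open and closed by itself on a repeating cycle, with no player interaction.
; Tick feeds a two-second Delay into a FlipFlop that alternately plays and reverses the Door timeline driving Pivot yaw.
; Opening also runs a second timeline that pitches the Knob.
; Two cross-resetting DoOnce nodes alternate the open and close sounds, both played at world origin rather than the door.
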(event EventBeginPlay)

(event Collision|EventActorBeginOverlap
  (params (OtherActor :type Actor%20Object%20Reference)))

(event EventTick
  (params (DeltaSeconds :type Float%20%28single-precision%29))
  (Utilities|FlowControl|Delay 2.0)
  (Utilities|FlowControl|FlipFlop
    (:A
      (Utilities|FlowControl|Sequence
        (:then_0
          (bind _newtrack_0 (Timeline|Door Play)
            (:Update
              (Transformation|SetRelativeRotation (Variables|Default|GetPivot) (Math|Rotator|MakeRotator 0.0 0.0 _newtrack_0) false false))))
        (:then_1
          (Utilities|FlowControl|DoOnce false :!label _label
            (:Completed
              (Audio|PlaySoundatLocation "/Game/Tello/Sounds/S_OpenDoor.S_OpenDoor" "0, 0, 0" "0, 0, 0" 1.0 1.0 0.0 0 0 0 0)
              (goto _label_2 Reset))))
        (:then_2
          (bind _newtrack_0_2 (Timeline|Timeline PlayFromStart)
            (:Update
              (Transformation|SetRelativeRotation (Variables|Default|GetKnob) (Math|Rotator|MakeRotator 0.0 _newtrack_0_2 0.0) false false))))))
    (:B
      (Utilities|FlowControl|Sequence
        (:then_0
          (Timeline|Door Reverse))
        (:then_1
          (Utilities|FlowControl|DoOnce false :!label _label_2
            (:Completed
              (Audio|PlaySoundatLocation "/Game/Tello/Sounds/S_CloseDoor.S_CloseDoor" "0, 0, 0" "0, 0, 0" 1.0 1.0 0.0 0 0 0 0)
              (goto _label Reset))))))))

(fn ConstructionScript)